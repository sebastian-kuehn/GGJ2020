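; EMP actor in the game's Ending content that destroys Launcher actors with a spherical pulse.
; Each Tick sets actor scale to the sphere's world scale times DeltaSeconds, removing the sphere component if that X value reaches a large threshold.
; Sphere overlap events scan all Launchers, destroying any that pass an overlap check with a small toon explosion and sound.
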(event OnComponentBeginOverlap(Sphere_EMP)
  (params (OverlappedComponent :type Primitive%20Component%20Object%20Reference) (OtherActor :type Actor%20Object%20Reference) (OtherComp :type Primitive%20Component%20Object%20Reference) (OtherBodyIndex :type Integer) (bFromSweep :type Boolean) (SweepResult :type Hit%20Result%20Structure%20%28by%20ref%29))
  (bind _outactors (Actor|GetAllActorsOfClass "/Game/GameJam/Blueprints/AI/Launcher.Launcher_C"))
  (for _index (range 0 (- (Utilities|Array|Length _outactors) 1))
    (if (Collision|IsOverlappingActor (Utilities|Array|Get(acopy) _outactors _index) 0 :!class /Script/Engine.Actor)
      (Effects|SpawnEmitteratLocation "/Game/GameJam/Art/Emitter/FirstPersonBP/ToonExplosion.ToonExplosion" (Transformation|GetActorLocation (Utilities|Array|Get(acopy) _outactors _index)) "0, 0, 0" "0.200000,0.200000,0.200000")
      (Audio|PlaySoundatLocation "/Game/GameJam/Audio/SFX/Cue_Explosion.Cue_Explosion" (Transformation|GetActorLocation (Utilities|Array|Get(acopy) _outactors _index)) "0, 0, 0" 1.0 1.0 0.0 0 0 0)
      (Actor|DestroyActor (Utilities|Array|Get(acopy) _outactors _index)))))

(event EventBeginPlay)

(event EventTick
  (params (DeltaSeconds :type Float%20%28single-precision%29))
  (bind _sphere_emp (Variables|Default|GetSphere_EMP))
  (bind _returnvalue (Transformation|GetWorldScale _sphere_emp))
  (bind _returnvalue_2 (* _returnvalue DeltaSeconds))
  (Transformation|SetActorScale3D _returnvalue_2)
  (if (>= (.X (Math|Vector|BreakVector _returnvalue_2)) 1.5e+03)
    (Components|DestroyComponent _sphere_emp)))

(fn ConstructionScript)