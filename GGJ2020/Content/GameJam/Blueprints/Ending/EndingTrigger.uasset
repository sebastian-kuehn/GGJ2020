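; EndingTrigger is a trigger actor that starts the game's ending by setting off an EMP at a golem's position.
; When its Trigger component is overlapped, it loops over all BP_Golem actors and runs an overlap check on each.
; Each golem that passes gets a CommenceEnding call, which spawns and stores an EMP actor at that location and plays the EMP sound there.
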(event OnComponentBeginOverlap(Trigger)
  (params (OverlappedComponent :type Primitive%20Component%20Object%20Reference) (OtherActor :type Actor%20Object%20Reference) (OtherComp :type Primitive%20Component%20Object%20Reference) (OtherBodyIndex :type Integer) (bFromSweep :type Boolean) (SweepResult :type Hit%20Result%20Structure%20%28by%20ref%29))
  (bind _outactors (Actor|GetAllActorsOfClass "/Game/GameJam/Blueprints/Character/GolemAI/BP_Golem.BP_Golem_C"))
  (for _index (range 0 (- (Utilities|Array|Length _outactors) 1))
    (if (Collision|IsOverlappingActor (Utilities|Array|Get(acopy) _outactors _index) 0 :!class /Script/Engine.Actor)
      (bind _output_get (Variables|Default|SetGolem_Location (Transformation|GetActorLocation (Utilities|Array|Get(acopy) _outactors _index))))
      (CallFunction|CommenceEnding _output_get))))

(event EventBeginPlay)

(event Collision|EventActorBeginOverlap
  (params (OtherActor :type Actor%20Object%20Reference)))

(event EventTick
  (params (DeltaSeconds :type Float%20%28single-precision%29)))

(fn ConstructionScript)

(fn CommenceEnding
  (params (Location :type Vector))
  (bind _returnvalue (Game|SpawnActorfromClass "/Game/GameJam/Blueprints/Ending/EMP.EMP_C" (Math|Conversions|ToTransform(Vector) Location) "AlwaysSpawn" 0 0))
  (Variables|Default|SetEMP _returnvalue)
  ;[1 1 1] Sound einfügen
  (Audio|PlaySoundatLocation "/Game/GameJam/Audio/SFX/Cue_EMP.Cue_EMP" Location "0, 0, 0" 1.0 1.0 0.0 0 0 0))