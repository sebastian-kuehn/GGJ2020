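; BP_Missile_of_nuclear_justice is a homing missile aimed at one of six random hit points on BP_Golem.
; BeginPlay picks the point, and Tick re-reads its location, eases the missile toward it with VInterpTo and spawns a marker particle there.
; On overlapping a drone it applies damage and destroys itself, skipping the explosion if the drone is shielding.
; The golem branch explodes and self-destructs, but its ApplyDamage call has no target set.
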(event Collision|EventActorBeginOverlap
  (params (OtherActor :type Actor%20Object%20Reference))
  (bind _mesh (Variables|Character|GetMesh))
  (bind _returnvalue (Transformation|GetWorldLocation _mesh))
  (Utilities|Casting|CastToBP_Golem OtherActor
    (:then
      (Development|PrintString "BOOOM")
      (Game|Damage|ApplyDamage 0 2e+01 0 0)
      (Effects|SpawnEmitteratLocation "/Game/GameJam/Art/Emitter/FirstPersonBP/ToonExplosion.ToonExplosion" _returnvalue "0, 0, 0" (Variables|Default|GetExplosionScale))
      (Actor|DestroyActor))
    (:CastFailed
      (bind _asbp_drone (Utilities|Casting|CastToBP_Drone OtherActor))
      (Game|Damage|ApplyDamage _asbp_drone 2e+01 0 0)
      (switch Utilities|FlowControl|Switch|SwitchonE_DroneState (Variables|/Game/GameJam/Blueprints/Character/BP_Drone.BP_Drone_C|GetState _asbp_drone)
        (:NewEnumerator2
          (Effects|SpawnEmitteratLocation "/Game/GameJam/Art/Emitter/FirstPersonBP/ToonExplosion.ToonExplosion" _returnvalue :!label _label)
          (Development|PrintString "Batsch")
          (Actor|DestroyActor))
        (:NewEnumerator0
          (goto _label))
        (:NewEnumerator1
          (Development|PrintString "Batsch")
          (Actor|DestroyActor))))))

(event EventTick
  (params (DeltaSeconds :type Float%20%28single-precision%29))
  (Utilities|FlowControl|Sequence
    (:then_0
      (switch int (Variables|Default|GetRandomHit)
        (:0
          (Utilities|SetImpactPoint (Variables|/Game/GameJam/Blueprints/Character/GolemAI/BP_Golem.BP_Golem_C|GetHeadHit (Variables|Default|GetGolem))))
        (:1
          (Utilities|SetImpactPoint (Variables|/Game/GameJam/Blueprints/Character/GolemAI/BP_Golem.BP_Golem_C|GetTorsorHit (Variables|Default|GetGolem))))
        (:2
          (Utilities|SetImpactPoint (Variables|/Game/GameJam/Blueprints/Character/GolemAI/BP_Golem.BP_Golem_C|GetLeftArmHit (Variables|Default|GetGolem))))
        (:3
          (Utilities|SetImpactPoint (Variables|/Game/GameJam/Blueprints/Character/GolemAI/BP_Golem.BP_Golem_C|GetRightArmHit (Variables|Default|GetGolem))))
        (:4
          (Utilities|SetImpactPoint (Variables|/Game/GameJam/Blueprints/Character/GolemAI/BP_Golem.BP_Golem_C|GetLeftKneeHit (Variables|Default|GetGolem))))
        (:5
          (Utilities|SetImpactPoint (Variables|/Game/GameJam/Blueprints/Character/GolemAI/BP_Golem.BP_Golem_C|GetRightKneeHit (Variables|Default|GetGolem))))))
    (:then_1
      (Transformation|SetActorLocation (Math|Interpolation|VInterpTo (Transformation|GetActorLocation) (Variables|Default|GetImpactPoint) DeltaSeconds 1.0) false false)
      (Effects|SpawnEmitteratLocation "/Engine/Tutorial/SubEditors/TutorialAssets/TutorialParticleSystem.TutorialParticleSystem" (Variables|Default|GetImpactPoint)))))

(event EventBeginPlay
  (bind _outactors (Actor|GetAllActorsOfClass "/Game/GameJam/Blueprints/Character/GolemAI/BP_Golem.BP_Golem_C"))
  (for _array_element _outactors
    (Variables|Default|SetGolem _array_element)
    (Variables|Default|SetRandomHit (Math|Random|RandomIntegerinRange 0 5))))

(fn ConstructionScript)