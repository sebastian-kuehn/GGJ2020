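; Behavior tree task that picks the next move location for a BP_Missile_of_nuclear_justice pawn.
; With a valid PatrolPath, it converts the path point at the blackboard's path index to world space and writes it to the move location key.
; Otherwise it writes the player character's current location, then finishes successfully in both cases.
; It does not advance the index, and a failed cast leaves the task without calling FinishExecute.
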(event EventReceiveExecuteAI
  (params (OwnerController :type AI%20Controller%20Object%20Reference) (ControlledPawn :type Pawn%20Object%20Reference))
  (bind _asbp_missile_of_nuclear_justice (Utilities|Casting|CastToBP_Missile_of_nuclear_justice ControlledPawn))
  (bind _patrolpath (Variables|/Game/GameJam/Blueprints/AI/BP_Missile_of_nuclear_justice.BP_Missile_of_nuclear_justice_C|GetPatrolPath _asbp_missile_of_nuclear_justice)
    (:then
      (Development|PrintString "guided")
      (AI|BehaviorTree|SetBlackboardValueasVector (Variables|Default|GetMoveLocationKey) (Math|Transform|TransformLocation (Transformation|GetActorTransform _patrolpath) (Utilities|Array|Get(acopy) (Variables|/Game/GameJam/Blueprints/AI/BP_Patrol_Points.BP_Patrol_Points_C|GetPathPoints _patrolpath) (Class|BTFunctionLibrary|GetBlackboardValueasInt (Variables|Default|GetPathIndexKey))))))
    (:else
      (Development|PrintString "straigt")
      (bind _asthird_person_character (Utilities|Casting|CastToThirdPersonCharacter (Game|GetPlayerCharacter 0)))
      (AI|BehaviorTree|SetBlackboardValueasVector (Variables|Default|GetMoveLocationKey) (Transformation|GetActorLocation _asthird_person_character))))
  (AI|BehaviorTree|FinishExecute true))