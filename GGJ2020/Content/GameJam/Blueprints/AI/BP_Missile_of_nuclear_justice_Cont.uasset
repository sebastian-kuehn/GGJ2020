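; AI controller for the Missile of nuclear justice pawn that drives its behavior tree.
; On possession it runs BT_Missile_of_nuclear_justice if the pawn is that missile type.
; Each tick it copies the missile's ImpactPoint into the GolemLocation blackboard key, while an isAttacking? blackboard write is left unconnected.
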(event EventPossess
  (params (PossessedPawn :type Pawn%20Object%20Reference))
  (Utilities|Casting|CastToBP_Missile_of_nuclear_justice PossessedPawn)
  (AI|RunBehaviorTree "/Game/GameJam/Blueprints/AI/BT_Missile_of_nuclear_justice.BT_Missile_of_nuclear_justice"))

(event EventTick
  (params (DeltaSeconds :type Float%20%28single-precision%29))
  (bind _asbp_missile_of_nuclear_justice (Utilities|Casting|CastToBP_Missile_of_nuclear_justice (Pawn|GetControlledPawn)))
  (AI|Components|Blackboard|SetValueasVector (AI|GetBlackboard 0) (Utilities|Name|MakeLiteralName "GolemLocation") (Variables|/Game/GameJam/Blueprints/AI/BP_Missile_of_nuclear_justice.BP_Missile_of_nuclear_justice_C|GetImpactPoint _asbp_missile_of_nuclear_justice)))

(fn ConstructionScript)