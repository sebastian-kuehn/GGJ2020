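; Missile launcher Actor that fires BP_Missile_of_nuclear_justice while something overlaps its sphere collision.
; Sphere overlap begin and end toggle IsActive, which Tick checks after a one-second Delay.
; Each active check calls SpawnMissile and restarts its looping timer, which is never cleared and keeps firing after deactivation.
; SpawnMissile spawns the missile just above the mesh with an explosion effect and rocket sound.
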(event OnComponentBeginOverlap(SphereCollision)
  (params (OverlappedComponent :type Primitive%20Component%20Object%20Reference) (OtherActor :type Actor%20Object%20Reference) (OtherComp :type Primitive%20Component%20Object%20Reference) (OtherBodyIndex :type Integer) (bFromSweep :type Boolean) (SweepResult :type Hit%20Result%20Structure%20%28by%20ref%29))
  (Variables|Default|SetisActive true))

(event OnComponentEndOverlap(SphereCollision)
  (params (OverlappedComponent :type Primitive%20Component%20Object%20Reference) (OtherActor :type Actor%20Object%20Reference) (OtherComp :type Primitive%20Component%20Object%20Reference) (OtherBodyIndex :type Integer))
  (Variables|Default|SetisActive false))

(event EventBeginPlay)

(event Collision|EventActorBeginOverlap
  (params (OtherActor :type Actor%20Object%20Reference)))

(event EventTick
  (params (DeltaSeconds :type Float%20%28single-precision%29))
  (Utilities|FlowControl|Delay 1.0)
  (if (Variables|Default|GetisActive)
    (Utilities|Time|SetTimerbyFunctionName 0 "SpawnMissile" 15.0 true 2.0)
    (CallFunction|SpawnMissile)))

(fn ConstructionScript)

(fn SpawnMissile
  (bind _mesh (Variables|Default|GetMesh))
  (bind _returnvalue (Transformation|GetWorldLocation _mesh))
  (bind _returnvalue_2 (+ _returnvalue "0, 0,10.000000"))
  (Game|SpawnActorfromClass "/Game/GameJam/Blueprints/AI/BP_Missile_of_nuclear_justice.BP_Missile_of_nuclear_justice_C" (Math|Conversions|ToTransform(Vector) _returnvalue_2) "AlwaysSpawn" 0 0)
  (Effects|SpawnEmitteratLocation "/Game/GameJam/Art/Emitter/FirstPersonBP/ToonExplosion.ToonExplosion" _returnvalue_2 "0, 0, 0" "2.000000,2.000000,2.000000")
  ;[1 1 1] Sound einfügen
  (Audio|PlaySoundatLocation "/Game/GameJam/Audio/SFX/Cue_Rocketshot.Cue_Rocketshot" _returnvalue_2 "0, 0, 0" 1.0 1.0 0.0 0 0 0))