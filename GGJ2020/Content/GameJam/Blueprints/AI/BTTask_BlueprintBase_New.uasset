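; Behavior Tree task that switches the nuclear justice missile pawn into attack mode when its patrol path runs out.
; On AI execute, it compares the Blackboard patrol index against the number of points in the missile's PatrolPath.
; While points remain it only prints the index; otherwise it sets IsAttacking and prints a debug message.
; Both branches finish successfully, and the task itself neither moves the pawn nor advances the index.
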(event EventReceiveExecuteAI
  (params (OwnerController :type AI%20Controller%20Object%20Reference) (ControlledPawn :type Pawn%20Object%20Reference))
  (bind _asbp_missile_of_nuclear_justice (Utilities|Casting|CastToBP_Missile_of_nuclear_justice ControlledPawn))
  (if (> (Utilities|Array|Length (Variables|/Game/GameJam/Blueprints/AI/BP_Patrol_Points.BP_Patrol_Points_C|GetPathPoints (Variables|/Game/GameJam/Blueprints/AI/BP_Missile_of_nuclear_justice.BP_Missile_of_nuclear_justice_C|GetPatrolPath _asbp_missile_of_nuclear_justice))) (Class|BTFunctionLibrary|GetBlackboardValueasInt (Variables|Default|GetPatrolPathKey)))
    (Development|PrintString (Utilities|String|ToString(Integer) (Class|BTFunctionLibrary|GetBlackboardValueasInt (Variables|Default|GetPatrolPathKey))))
    (else
      (bind _asbp_missile_of_nuclear_justice_2 (Utilities|Casting|CastToBP_Missile_of_nuclear_justice ControlledPawn))
      (Variables|/Game/GameJam/Blueprints/AI/BP_Missile_of_nuclear_justice.BP_Missile_of_nuclear_justice_C|SetisAttacking? _asbp_missile_of_nuclear_justice_2 true)
      (Development|PrintString "attack")))
  (AI|BehaviorTree|FinishExecute true))